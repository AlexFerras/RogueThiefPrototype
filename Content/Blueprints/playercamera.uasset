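; Player camera pawn that handles mouse selection and grid-based movement of characters.
; Each tick it traces under the cursor and, when the hit actor's hover message returns true, has the selected character show a path to each newly hovered grid cell.
; Clicks select characters through interface messages, unclicking the previous one, or otherwise move the selection to a cell within its drawn points, then clear the path.
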(event EventBeginPlay
  (bind _asplayer_controller (Utilities|Casting|CastToPlayerController (Pawn|GetController)))
  (Variables|Default|SetPC _asplayer_controller))

(event Collision|EventActorBeginOverlap
  (params (OtherActor :type Actor%20Object%20Reference)))

(event EventTick
  (params (DeltaSeconds :type Float%20%28single-precision%29))
  (bind _pc (Variables|Default|GetPC))
  (bind _character (Variables|Default|GetCharacter))
  (bind _hitresult (Game|Player|GetHitResultUnderCursorbyChannel _pc "TraceTypeQuery2" true))
  (bind _returnvalue (Class|GridFunctionLib|ConvertWorldtoGrid (.location _hitresult)))
  (bind _result (Class|BPISelection|HoverBPI(Message) (.hitactor _hitresult)))
  (if _result
    (Utilities|IsValid _character
      (:Is%20Valid
        (if (not (Class|GridFunctionLib|IsEqual _returnvalue (Variables|Default|GetPosition)))
          (bind _output_get (Variables|Default|SetPosition _returnvalue))
          (Default|ShowPath _character _output_get))))))

(event Input|ActionEvents|InputActionPrimaryMouse
  (params (Key :type Key%20Structure :default "None"))
  (bind _pc (Variables|Default|GetPC))
  (bind _hitresult (Game|Player|GetHitResultUnderCursorbyChannel _pc "TraceTypeQuery2" true))
  (bind _returnvalue (Class|GridFunctionLib|ConvertWorldtoGrid (.location _hitresult)))
  (:Pressed
    (bind _result (Class|BPISelection|ClickBPI(Message) (.hitactor _hitresult) self))
    (if _result
      (Utilities|IsValid (Variables|Default|GetCharacter)
        (:Is%20Valid
          (if (!= (.hitactor _hitresult) (Variables|Default|GetCharacter))
            (Class|BPISelection|UnclickBPI(Message) (Variables|Default|GetCharacter))))
        (:Is%20Not%20Valid
          _))
      (bind _asthird_person_character (Utilities|Casting|CastToThirdPersonCharacter (.hitactor _hitresult)))
      (Variables|Default|SetCharacter _asthird_person_character)
      (else
        (Utilities|IsValid (Variables|Default|GetCharacter)
          (:Is%20Valid
            (if (Utilities|Array|ContainsItem (Variables|/Game/ThirdPersonBP/Blueprints/ThirdPersonCharacter.ThirdPersonCharacter_C|GetDrawedPoints (Variables|Default|GetCharacter)) _returnvalue)
              (Default|MoveonVectors (Variables|Default|GetCharacter) _returnvalue)
              (Default|HidePath (Variables|Default|GetCharacter))
              (Default|DeletePoints (Variables|Default|GetCharacter)))))))))

(fn ConstructionScript)

(fn GetCameraLocation
  (return (Transformation|GetWorldLocation (Variables|Default|GetCamera))))
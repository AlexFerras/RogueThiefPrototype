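; BP_Blockbox is a grid-based block actor that identifies as a block rather than a wall.
; Shortly after BeginPlay it passes its world position, converted to grid coordinates, to its Grid's MoveOnGrid, while SetToGrid snaps it by round-trip conversion.
; Tick writes the grid position to a TextRender in Z, X, Y order.
; Its interface functions return true for click and false for hover and unclick.
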(event Custom|SetToGrid
  (Transformation|SetActorLocation (Class|GridFunctionLib|ConvertGridtoWorld (Class|GridFunctionLib|ConvertWorldtoGrid (Transformation|GetActorLocation))) false false))

(event EventBeginPlay
  (Utilities|FlowControl|Delay 0.2)
  (Class|GridComponent|MoveonGrid (Variables|Default|GetGrid) (Class|GridFunctionLib|ConvertWorldtoGrid (Transformation|GetActorLocation))))

(event Collision|EventActorBeginOverlap
  (params (OtherActor :type Actor%20Object%20Reference)))

(event EventTick
  (params (DeltaSeconds :type Float%20%28single-precision%29))
  (bind _returnvalue (Class|GridComponent|GetGridPosition (Variables|Default|GetGrid)))
  (Rendering|Components|TextRender|SetText (Variables|Default|GetTextRender) (Utilities|Text|FormatText "{1}, {2}, {3}" (.z _returnvalue) (.x _returnvalue) (.y _returnvalue))))

(fn ConstructionScript)

(fn ClickBPI
  (params (Camera :type Tactical%20Player%20Camera%20Object%20Reference))
  (return true))

(fn HoverBPI
  (return false))

(fn IsBlock
  (return true))

(fn IsWall
  (return "" "" false))

(fn UnclickBPI
  (return false))
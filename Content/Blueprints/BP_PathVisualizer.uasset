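; Debug visualizer for grid-based pathfinding that marks results in the world with spawned actors.
; BeginPlay converts the StartPoint and TargetPoint actor locations into grid Start and Target coordinates.
; PrintPath spawns a slightly raised Path actor at each path cell, and PrintStraight spawns a Point actor at a given cell.
; PrintCurrentNode is empty, with a direction-marker spawn left disconnected.
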(event EventPrintStraight
  (params (Pos :type Grid%20Vector%20Structure%20%28by%20ref%29))
  (Game|SpawnActorfromClass "/Game/Blueprints/Point.Point_C" (Math|Transform|MakeTransform (Class|GridFunctionLib|ConvertGridtoWorld Pos) "0, 0, 0" "1,1,1") "Undefined" 0 "0.000000,0.000000,0.000000" 0))

(event Collision|EventActorBeginOverlap
  (params (OtherActor :type Actor%20Object%20Reference)))

(event EventTick
  (params (DeltaSeconds :type Float%20%28single-precision%29)))

(event EventPrintCurrentNode
  (params (Position :type Grid%20Vector%20Structure%20%28by%20ref%29) (DirectionToParent :type Vector%20%28by%20ref%29 :default "0, 0, 0")))

(event EventPrintPath
  (params (Path :type Grid%20Path%20Structure%20%28by%20ref%29))
  (for _array_element (Class|GridFunctionLib|ToArray Path)
    (Game|SpawnActorfromClass "/Game/Blueprints/Path.Path_C" (Math|Transform|MakeTransform (+ (Class|GridFunctionLib|ConvertGridtoWorld _array_element) "0, 0,5.000000") "0, 0, 0" "1,1,1") "Undefined" 0 0)))

(event EventBeginPlay
  (Variables|Default|SetStart (Class|GridFunctionLib|ConvertWorldtoGrid (Transformation|GetActorLocation (Variables|Settings|GetStartPoint))))
  (Variables|Default|SetTarget (Class|GridFunctionLib|ConvertWorldtoGrid (Transformation|GetActorLocation (Variables|Settings|GetTargetPoint)))))

(fn ConstructionScript)
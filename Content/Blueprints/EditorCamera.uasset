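; EditorCamera is the player-controlled camera for an in-game editor that places and removes actors with the mouse.
; BeginPlay opens the UI_Editor widget in game-and-UI input mode, and ItemSelected stores the class to place.
; Tick sends an interface hover message to the actor under the cursor.
; A primary click sends a click message, destroying the hit actor on a true reply, otherwise spawning the selected class at the hit location.
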(event EventBeginPlay
  (bind _asplayer_controller (Utilities|Casting|CastToPlayerController (Pawn|GetController)))
  (bind _output_get (Variables|Default|SetPC _asplayer_controller))
  (bind _returnvalue (UserInterface|CreateWidget "/Game/Blueprints/UI_Editor.UI_Editor_C" _output_get))
  (UserInterface|Viewport|AddtoViewport _returnvalue 0)
  (Input|SetInputModeGameandUI _output_get _returnvalue "DoNotLock" false))

(event Collision|EventActorBeginOverlap
  (params (OtherActor :type Actor%20Object%20Reference)))

(event EventTick
  (params (DeltaSeconds :type Float%20%28single-precision%29))
  (Class|BPISelection|HoverBPI(Message) (.hitactor (.HitResult (Game|Player|GetHitResultUnderCursorbyChannel (Variables|Default|GetPC) "TraceTypeQuery2" false)))))

(event Input|ActionEvents|InputActionPrimaryMouse
  (params (Key :type Key%20Structure :default "None"))
  (bind _pc (Variables|Default|GetPC))
  (bind _hitresult (Game|Player|GetHitResultUnderCursorbyChannel _pc "TraceTypeQuery1" true))
  (:Pressed
    (bind _result (Class|BPISelection|ClickBPI(Message) (.hitactor _hitresult) self))
    (if _result
      (Actor|DestroyActor (.hitactor _hitresult))
      (else
        (Game|SpawnActorfromClass (Utilities|ResolveSoftReference (Variables|Default|GetCurrentItemClass)) (Math|Transform|MakeTransform (.location _hitresult) "0, 0,0.000000" "1,1,1") "Undefined" 0 0)))))

(fn ConstructionScript)

(fn GetCameraLocation
  (return (Transformation|GetWorldLocation (Variables|Default|GetCamera))))

(fn ItemSelected
  (params (Class :type Actor%20Soft%20Class%20Reference))
  (Variables|Default|SetCurrentItemClass Class))
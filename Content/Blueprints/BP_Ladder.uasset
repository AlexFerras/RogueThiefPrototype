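; BP_Ladder is a grid-placed ladder that acts as both a wall and a connector between grid positions.
; SetToGrid snaps its location to the grid with a slight Z lift, aligns its rotation, then updates its GridConnector component.
; Interface queries report wall positions from GridWall and the connected position from GridConnector, while denying being a block or floor.
; It returns true for clicks and false for hover and unclick.
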(event Custom|SetToGrid
  (Transformation|SetActorLocation (+ (Class|GridFunctionLib|ConvertGridtoWorld (Class|GridFunctionLib|ConvertWorldtoGrid (Transformation|GetActorLocation))) "0, 0,1.000000") false false)
  (Transformation|SetActorRotation (Class|GridFunctionLib|GetRotationtoGrid (Transformation|GetActorForwardVector)))
  (Class|GridConnectorComponent|SettoGrid (Variables|Default|GetGridConnector)))

(event EventBeginPlay)

(event Collision|EventActorBeginOverlap
  (params (OtherActor :type Actor%20Object%20Reference)))

(event EventTick
  (params (DeltaSeconds :type Float%20%28single-precision%29)))

(fn ConstructionScript)

(fn ClickBPI
  (params (Camera :type Tactical%20Player%20Camera%20Object%20Reference))
  (return true))

(fn HoverBPI
  (return false))

(fn IsBlock
  (return false))

(fn IsConnector
  (params (Pos :type Grid%20Vector%20Structure%20%28by%20ref%29))
  (return (Class|GridConnectorComponent|GetConnectedPos (Variables|Default|GetGridConnector) Pos) true))

(fn IsFloor
  (return 0 false))

(fn IsWall
  (bind (_pos1 _pos2) (Class|GridWallComponent|GetGridPosition (Variables|Default|GetGridWall)))
  (return _pos1 _pos2 true))

(fn UnclickBPI
  (return false))